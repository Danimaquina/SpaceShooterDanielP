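; Drone enemy for the space shooter that moves along a movement vector and fires paired left and right bullets.
; Tick moves it without sweep and runs a timer that calls Fire1 and Fire2, each spawning a bullet at its fire point and setting its direction.
; Overlapping a "Caida" tag reverses movement.
; Player contact triggers an explosion, notifies the game mode, damages the player and destroys the drone.
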(event `self.ReceiveActorBeginOverlap`
  (params (OtherActor :type "Actor Object Reference"))
  (if (`KismetArrayLibrary.Array_Contains` (`Actor.Tags` OtherActor) "Player")
    (`GameplayStatics.SpawnEmitterAtLocation` "/Game/StarterContent/Particles/P_Explosion.P_Explosion" (`self.K2_GetActorLocation`))
    (bind _asss_game_mode (cast `/Game/00_Space_Shooter/SS_GameMode` (`GameplayStatics.GetGameMode`)))
    (`/Game/00_Space_Shooter/SS_GameMode.EnemyDestroyed` _asss_game_mode)
    (bind _asss_player_character (cast `/Game/00_Space_Shooter/Player/SS_Player_Character` (`GameplayStatics.GetPlayerCharacter` 0)))
    (`/Game/00_Space_Shooter/Player/SS_Player_Character.Damage` _asss_player_character)
    (`self.K2_DestroyActor`)
    (elif (`KismetArrayLibrary.Array_Contains` (`Actor.Tags` OtherActor) "Caida")
      (set `self.MovementVector` (* (`self.MovementVector`) (-1.0 -1.0 -1.0))))))

(event `self.ReceiveTick`
  (params (DeltaSeconds :type "Float (single-precision)"))
  ;[1 1 1] Comment
  (`self.K2_SetActorLocation` (+ (`self.K2_GetActorLocation`) (* (* DeltaSeconds (`self.Speed`)) (`self.MovementVector`))))
  (set `self.ShootCurrentTime` (+ (`self.ShootCurrentTime`) DeltaSeconds))
  (if (> (`self.ShootCurrentTime`) (`self.DelayShoot`))
    (`self.Fire1`)
    (`self.Fire2`)
    (set `self.ShootCurrentTime` 0.0)))

(fn `Fire1`
  (bind _returnvalue (`|SpawnActorFromClass` "/Game/00_Space_Shooter/Enemies/EnemyBulletIZQUIERDA.EnemyBulletIZQUIERDA_C" (`SceneComponent.K2_GetComponentToWorld` (`self.FirePoint`)) "Undefined" "OverrideRootScale" null null))
  (bind _output_get (set `self.bullet1` _returnvalue))
  (`/Game/00_Space_Shooter/Enemies/EnemyBullet.SetBulletDirection` _output_get)
  (set `/Game/00_Space_Shooter/Enemies/EnemyBullet.DirectionBullet` "NewEnumerator2" (`self.bullet1`)))

(fn `Fire2`
  (bind _returnvalue (`|SpawnActorFromClass` "/Game/00_Space_Shooter/Enemies/EnemyBulletDERECHA.EnemyBulletDERECHA_C" (`SceneComponent.K2_GetComponentToWorld` (`self.FirePoint3`)) "Undefined" "MultiplyWithRoot" null null))
  (bind _output_get (set `self.bullet2` _returnvalue))
  (`/Game/00_Space_Shooter/Enemies/EnemyBullet.SetBulletDirection` _output_get)
  (set `/Game/00_Space_Shooter/Enemies/EnemyBullet.DirectionBullet` "NewEnumerator1" (`self.bullet2`)))

(fn `UserConstructionScript`
  (`parent.UserConstructionScript`))