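; Base enemy actor for the space shooter that flies along its initial forward vector and attacks on a timer.
; When able to fire, it shoots a bullet or, as a bomber, drops a bomb.
; Overlapping Player or "Caida" actors makes it explode and notify the game mode, damaging the player in the first case.
; It also provides weighted-random power-up drops and a look-at-player helper, neither called in this graph.
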(event `self.ReceiveBeginPlay`
  (set `self.MovementVector` (`self.GetActorForwardVector`)))

(event `self.ReceiveTick`
  (params (DeltaSeconds :type "Float (single-precision)"))
  ;[1 1 1] Comment
  (`self.K2_SetActorLocation` (+ (`self.K2_GetActorLocation`) (* (* DeltaSeconds (`self.Speed`)) (`self.MovementVector`))))
  (if (`self.CanFire`)
    (set `self.ShootCurrentTime` (+ (`self.ShootCurrentTime`) DeltaSeconds))
    (if (> (`self.ShootCurrentTime`) (`self.DelayShoot`))
      (if (`self.Bombardero`)
        (`self.Plantar`)
        (set `self.ShootCurrentTime` 0.0)
        (else
          (`self.Fire`)
          (set `self.ShootCurrentTime` 0.0))))))

(event `self.ReceiveActorBeginOverlap`
  (params (OtherActor :type "Actor Object Reference"))
  (if (`KismetArrayLibrary.Array_Contains` (`Actor.Tags` OtherActor) "Player")
    (`GameplayStatics.SpawnEmitterAtLocation` "/Game/StarterContent/Particles/P_Explosion.P_Explosion" (`self.K2_GetActorLocation`))
    (`GameplayStatics.PlaySound2D` "/Game/StarterContent/Audio/Explosion01.Explosion01" 1.0 1.0 0.0 null null)
    (bind _asss_player_character (cast `/Game/00_Space_Shooter/Player/SS_Player_Character` (`GameplayStatics.GetPlayerCharacter` 0)))
    (`/Game/00_Space_Shooter/Player/SS_Player_Character.Damage` _asss_player_character)
    (bind _asss_game_mode (cast `/Game/00_Space_Shooter/SS_GameMode` (`GameplayStatics.GetGameMode`)))
    (`/Game/00_Space_Shooter/SS_GameMode.EnemyDestroyed` _asss_game_mode)
    (`self.K2_DestroyActor`)
    (elif (`KismetArrayLibrary.Array_Contains` (`Actor.Tags` OtherActor) "Caida")
      (`GameplayStatics.SpawnEmitterAtLocation` "/Game/StarterContent/Particles/P_Explosion.P_Explosion" (`self.K2_GetActorLocation`))
      (`GameplayStatics.PlaySound2D` "/Game/StarterContent/Audio/Explosion01.Explosion01" 1.0 1.0 0.0 null null)
      (bind _asss_game_mode_2 (cast `/Game/00_Space_Shooter/SS_GameMode` (`GameplayStatics.GetGameMode`)))
      (`/Game/00_Space_Shooter/SS_GameMode.EnemyDestroyed` _asss_game_mode_2)
      (`self.K2_DestroyActor`))))

(event `SpawnPowerUp`
  (params (EscudosPosibility :type "Float (double-precision)") (MotoresPosibility :type "Float (double-precision)") (DisparosPosibility :type "Float (double-precision)") (ExplosionPosibility :type "Float (double-precision)") (NadaPosibility :type "Float (double-precision)"))
  (bind _output_get (set `self.RandomValue` (`KismetMathLibrary.RandomFloatInRange` 0.0 1.0)))
  (if (< _output_get NadaPosibility)
    _
    (elif (< (`self.RandomValue`) (+ NadaPosibility EscudosPosibility))
      (`|SpawnActorFromClass` "/Game/00_Space_Shooter/Player/SS_PowerUPShields.SS_PowerUPShields_C" (`SceneComponent.K2_GetComponentToWorld` (`self.Sphere`)) "Undefined" "MultiplyWithRoot" null null)
      (elif (< (`self.RandomValue`) (+ NadaPosibility EscudosPosibility MotoresPosibility))
        (`|SpawnActorFromClass` "/Game/00_Space_Shooter/Player/SS_PowerUPM+.SS_PowerUPM+_C" (`SceneComponent.K2_GetComponentToWorld` (`self.Sphere`)) "Undefined" "MultiplyWithRoot" null null)
        (elif (< (`self.RandomValue`) (+ NadaPosibility EscudosPosibility MotoresPosibility DisparosPosibility))
          (`|SpawnActorFromClass` "/Game/00_Space_Shooter/Player/SS_PowerUPS+.SS_PowerUPS+_C" (`SceneComponent.K2_GetComponentToWorld` (`self.Sphere`)) "Undefined" "MultiplyWithRoot" null null)
          (elif (< (`self.RandomValue`) (+ NadaPosibility EscudosPosibility MotoresPosibility DisparosPosibility ExplosionPosibility))
            (`|SpawnActorFromClass` "/Game/00_Space_Shooter/Player/SS_Nuke.SS_Nuke_C" (`SceneComponent.K2_GetComponentToWorld` (`self.Sphere`)) "Undefined" "MultiplyWithRoot" null null)))))))

(fn `Escaner`
  (`SceneComponent.K2_SetWorldRotation` (`self.Sphere`) (`KismetMathLibrary.FindLookAtRotation` (`SceneComponent.K2_GetComponentLocation` (`self.Sphere`)) (`SceneComponent.K2_GetComponentLocation` (`Character.Mesh` (`GameplayStatics.GetPlayerCharacter` 0)))) false false))

(fn `Fire`
  (bind _returnvalue (`|SpawnActorFromClass` "/Game/00_Space_Shooter/Enemies/EnemyBullet.EnemyBullet_C" (`SceneComponent.K2_GetComponentToWorld` (`self.FirePoint`)) "Undefined" "MultiplyWithRoot" null null))
  (bind _output_get (set `self.SpawnedBullet` _returnvalue))
  (`/Game/00_Space_Shooter/Enemies/EnemyBullet.SetBulletDirection` _output_get)
  (set `/Game/00_Space_Shooter/Enemies/EnemyBullet.DirectionBullet` "NewEnumerator0" (`self.SpawnedBullet`)))

(fn `Plantar`
  (`|SpawnActorFromClass` "/Game/00_Space_Shooter/Enemies/EnemyBomb.EnemyBomb_C" (`SceneComponent.K2_GetComponentToWorld` (`self.FirePoint`)) "Undefined" "MultiplyWithRoot" null null))

(fn `UserConstructionScript`)