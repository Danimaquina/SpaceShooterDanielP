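; Kamikaze enemy Blueprint for the space shooter that aims its movement at the player and does not fire.
; On BeginPlay it runs Escaner, then sets MovementVector once from its Sphere toward the player character's mesh, normalized before Z is zeroed.
; Tick forces CanFire to false before calling the parent Tick, leaving the remaining behavior to the parent class.
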(event `self.ReceiveBeginPlay`
  (`parent.ReceiveBeginPlay`)
  (`self.Escaner`)
  (set `self.MovementVector` (* (`KismetMathLibrary.Normal` (- (`SceneComponent.K2_GetComponentLocation` (`self.Sphere`)) (`SceneComponent.K2_GetComponentLocation` (`Character.Mesh` (`GameplayStatics.GetPlayerCharacter` 0))))) (-1.0 -1.0 0.0))))

(event `self.ReceiveTick`
  (params (DeltaSeconds :type "Float (single-precision)"))
  (set `self.CanFire` false)
  (`parent.ReceiveTick` DeltaSeconds))

(fn `UserConstructionScript`
  (`parent.UserConstructionScript`))